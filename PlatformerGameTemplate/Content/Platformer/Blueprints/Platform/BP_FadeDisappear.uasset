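; BP_FadeDisappear is a platform that fades and loses its collision after a BP_Character overlaps its trigger Box.
; BeginPlay puts a dynamic instance of M_Fade on the Cube.
; The overlap plays the Fade timeline into the material's Fade parameter, then disables Cube and Box collision when it finishes.
; An Active event restores the platform by setting Fade to one and both collisions to query-only.
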(event `self.ReceiveBeginPlay`
  (bind _returnvalue (`KismetMaterialLibrary.CreateDynamicMaterialInstance` "/Game/Platformer/Materials/M_Fade.M_Fade"))
  (bind _output_get (set `self.Mat` _returnvalue))
  (`PrimitiveComponent.SetMaterial` (`self.Cube`) 0 _output_get))

(event `self.Box.OnComponentBeginOverlap`
  (params (OverlappedComponent :type "PrimitiveComponent Object Reference") (OtherActor :type "Actor Object Reference") (OtherComp :type "PrimitiveComponent Object Reference") (OtherBodyIndex :type Integer) (bFromSweep :type Boolean) (SweepResult :type "HitResult Structure (by ref)"))
  (cast `/Game/Platformer/Blueprints/BP_Character` OtherActor)
  (bind (_direction _newtrack_0) (`Timeline|Fade` :!via `PlayFromStart`)
    (:`Update`
      (`MaterialInstanceDynamic.SetScalarParameterValue` (`self.Mat`) "Fade" _newtrack_0))
    (:`Finished`
      (`PrimitiveComponent.SetCollisionEnabled` (`self.Cube`) "NoCollision")
      (`PrimitiveComponent.SetCollisionEnabled` (`self.Box`) "NoCollision"))))

(event `Active`
  (`MaterialInstanceDynamic.SetScalarParameterValue` (`self.Mat`) "Fade" 1.0)
  (`PrimitiveComponent.SetCollisionEnabled` (`self.Cube`) "QueryOnly")
  (`PrimitiveComponent.SetCollisionEnabled` (`self.Box`) "QueryOnly"))

(fn `UserConstructionScript`)