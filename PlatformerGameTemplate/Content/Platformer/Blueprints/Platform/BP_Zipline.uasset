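; Bidirectional zipline actor that carries BP_Character along a spline between its two ends.
; BeginPlay snaps the second spline point just above the End component, and overlap boxes at either end set usability and travel direction.
; Use stops gliding, switches to Falling and plays a timeline forward or reversed, moving the character beneath the spline with matching yaw.
; LetGo, also called on finish, restores Walking and re-enables gliding.
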(event `/Game/Platformer/Blueprints/Interfaces/BPI_Zipline.LetGo`
  (bind _as_bp_character (`self.As BP Character`))
  (`TimelineComponent.Stop` (`self.Timeline_0`))
  (`self.MovementModeWalking`)
  (set `/Game/Platformer/Blueprints/BP_Character.As BP Zipline` null _as_bp_character)
  (set `/Game/Platformer/Blueprints/BP_Character.IsOnZipline` false _as_bp_character)
  (set `/Game/Platformer/Blueprints/BP_Character.CanGlide` true _as_bp_character))

(event `MovementModeWalking`
  (bind _as_bp_character (`self.As BP Character`))
  (`CharacterMovementComponent.SetMovementMode` (`Character.CharacterMovement` _as_bp_character) "MOVE_Walking" 0)
  (set `/Game/Platformer/Blueprints/BP_Character.Can Rotate` false _as_bp_character))

(event `self.Box1.OnComponentBeginOverlap`
  (params (OverlappedComponent :type "PrimitiveComponent Object Reference") (OtherActor :type "Actor Object Reference") (OtherComp :type "PrimitiveComponent Object Reference") (OtherBodyIndex :type Integer) (bFromSweep :type Boolean) (SweepResult :type "HitResult Structure (by ref)"))
  ;[1 1 1] Set Usable
  (bind _asbp_character (cast `/Game/Platformer/Blueprints/BP_Character` OtherActor))
  (set `self.As BP Character` _asbp_character)
  (set `self.Usable` true)
  ;;[1 1 1] BiDirectional
  (set `self.FromStart` false))

(event `self.Box.OnComponentBeginOverlap`
  (params (OverlappedComponent :type "PrimitiveComponent Object Reference") (OtherActor :type "Actor Object Reference") (OtherComp :type "PrimitiveComponent Object Reference") (OtherBodyIndex :type Integer) (bFromSweep :type Boolean) (SweepResult :type "HitResult Structure (by ref)"))
  ;[1 1 1] Set Usable
  (bind _asbp_character (cast `/Game/Platformer/Blueprints/BP_Character` OtherActor))
  (set `self.As BP Character` _asbp_character)
  (set `self.Usable` true)
  ;;[1 1 1] BiDirectional
  (set `self.FromStart` true))

(event `MovementModeFalling`
  (bind _as_bp_character (`self.As BP Character`))
  (`CharacterMovementComponent.SetMovementMode` (`Character.CharacterMovement` _as_bp_character) "MOVE_Falling" 0)
  (set `/Game/Platformer/Blueprints/BP_Character.Can Rotate` false _as_bp_character))

(event `self.Box1.OnComponentEndOverlap`
  (params (OverlappedComponent :type "PrimitiveComponent Object Reference") (OtherActor :type "Actor Object Reference") (OtherComp :type "PrimitiveComponent Object Reference") (OtherBodyIndex :type Integer))
  ;[1 1 1] Set Usable
  (cast `/Game/Platformer/Blueprints/BP_Character` OtherActor)
  (set `self.Usable` false)
  ;;[1 1 1] BiDirectional
  (set `self.FromStart` true))

(event `self.Box.OnComponentEndOverlap`
  (params (OverlappedComponent :type "PrimitiveComponent Object Reference") (OtherActor :type "Actor Object Reference") (OtherComp :type "PrimitiveComponent Object Reference") (OtherBodyIndex :type Integer))
  ;[1 1 1] Set Usable
  (cast `/Game/Platformer/Blueprints/BP_Character` OtherActor)
  (set `self.Usable` false)
  ;;[1 1 1] BiDirectional
  (set `self.FromStart` false))

(event `self.ReceiveBeginPlay`
  ;[1 1 1] Construction Script Alternative - Set path
  (`SplineComponent.SetLocationAtSplinePoint` (`self.Spline`) 1 (+ (`SceneComponent.K2_GetComponentLocation` (`self.End`)) (0.0 0.0 30.0)) "World" true))

(event `/Game/Platformer/Blueprints/Interfaces/BPI_Zipline.Use`
  (bind _spline (`self.Spline`))
  (bind _as_bp_character (`self.As BP Character`))
  ;[1 1 1] Follow Spline
  (if (`self.Usable`)
    (`/Game/Platformer/Blueprints/BP_Character.StopGliding` (`self.As BP Character`))
    (`self.MovementModeFalling`)
    (if (`self.FromStart`)
      (bind (_direction _newtrack_0) (`Timeline|Timeline_0` :!via `PlayFromStart` :!label _label)
        (:`Update`
          (if (`self.FromStart`)
            (bind _returnvalue (`KismetMathLibrary.Lerp` 0.0 (`SplineComponent.GetSplineLength` (`self.Spline`)) _newtrack_0))
            (bind (_returnvalue_x _returnvalue_y _returnvalue_z) (`KismetMathLibrary.BreakVector` (`SplineComponent.GetLocationAtDistanceAlongSpline` _spline _returnvalue "World")))
            (bind _returnvalue_2 (- _returnvalue_z 50.0))
            (bind (_returnvalue_roll _returnvalue_pitch _returnvalue_yaw) (`KismetMathLibrary.BreakRotator` (`SplineComponent.GetRotationAtDistanceAlongSpline` _spline _returnvalue "World")))
            (`self.K2_SetActorLocationAndRotation` _as_bp_character (`KismetMathLibrary.MakeVector` _returnvalue_x _returnvalue_y _returnvalue_2) (`KismetMathLibrary.MakeRotator` 0.0 0.0 _returnvalue_yaw) false false)
            (else
              (`self.K2_SetActorLocationAndRotation` _as_bp_character (`KismetMathLibrary.MakeVector` _returnvalue_x _returnvalue_y _returnvalue_2) (`KismetMathLibrary.MakeRotator` 0.0 0.0 _returnvalue_yaw) false false))))
        (:`Finished`
          (`/Game/Platformer/Blueprints/Interfaces/BPI_Zipline.LetGo`)))
      (else
        (goto _label :!via `ReverseFromEnd`)))))

(fn `UserConstructionScript`)