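; A rotating circular platform hazard for the platformer that hurts any BP_Character touching its two cylinders.
; A RotatingMovement component spins it, and the Reverse flag negates the rotation rate at BeginPlay.
; Each cylinder's overlap casts to BP_Character and calls SetHealth with a negative value, delayed one tick as a noted workaround for a destroy bug.
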(event `self.ReceiveBeginPlay`
  (bind _rotatingmovement (`self.RotatingMovement`))
  (if (`self.Reverse`)
    (set `RotatingMovementComponent.RotationRate` (`KismetMathLibrary.NegateRotator` (`RotatingMovementComponent.RotationRate` _rotatingmovement)) _rotatingmovement)))

(event `self.Cylinder.OnComponentBeginOverlap`
  (params (OverlappedComponent :type "PrimitiveComponent Object Reference") (OtherActor :type "Actor Object Reference") (OtherComp :type "PrimitiveComponent Object Reference") (OtherBodyIndex :type Integer) (bFromSweep :type Boolean) (SweepResult :type "HitResult Structure (by ref)"))
  (bind _asbp_character (cast `/Game/Platformer/Blueprints/BP_Character` OtherActor))
  ;[1 1 1] Bug Fix Dont Destroy
  (`KismetSystemLibrary.DelayUntilNextTick`)
  (`/Game/Platformer/Blueprints/BP_Character.SetHealth` _asbp_character -1.0))

(event `self.Cylinder1.OnComponentBeginOverlap`
  (params (OverlappedComponent :type "PrimitiveComponent Object Reference") (OtherActor :type "Actor Object Reference") (OtherComp :type "PrimitiveComponent Object Reference") (OtherBodyIndex :type Integer) (bFromSweep :type Boolean) (SweepResult :type "HitResult Structure (by ref)"))
  (bind _asbp_character (cast `/Game/Platformer/Blueprints/BP_Character` OtherActor))
  ;[1 1 1] Bug Fix Dont Destroy
  (`KismetSystemLibrary.DelayUntilNextTick`)
  (`/Game/Platformer/Blueprints/BP_Character.SetHealth` _asbp_character -1.0))

(fn `UserConstructionScript`)