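; Platformer obstacle actor that moves a set of small cubes around a square spline track at constant speed.
; BeginPlay builds the track from static meshes at edge midpoints and corners, then spawns the cubes and spaces them evenly by spline distance.
; Tick advances each cube's distance and repositions it slightly above the spline, resetting past the end when IsLooping is set.
; The construction script is empty, and an alternative spline-mesh track builder is left unconnected.
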(event `self.ReceiveBeginPlay`
  (set `self.SelectedSpline` (`self.SquareSpline`))
  (`self.AddSquareMesh`)
  ;[1 1 1] Add Cube
  (bind _result (`/Engine/EditorBlueprintResources/StandardMacros.DecrementInt` (`self.NumOfCubes`))
    (:`  `
      (for _index (range (+ _result 1))
        (bind _returnvalue (`AddComponent|NODE_AddStaticMeshComponent-0` :`RelativeTransform` (`KismetMathLibrary.MakeTransform` (0.0 0.0 0.0) (struct) (0.6 0.6 0.6))))
        (`BlueprintMapLibrary.Map_Add` (`self.CubeList`) _index _returnvalue)
        (`KismetArrayLibrary.Array_Add` (`self.Distance`))
        (`self.SetDistance`)))))

(event `self.ReceiveTick`
  (params (DeltaSeconds :type "Float (single-precision)"))
  (bind _distance (`self.Distance`))
  ;[1 1 1] CubeMovement
  (for _index (range (+ (`self.NumOfCubes`) 1))
    (bind _output (`|GetArrayItem` _distance _index))
    (`KismetArrayLibrary.Array_Set` _distance _index (+ (* DeltaSeconds (`self.Speed`)) _output))
    (bind (_returnvalue_x _returnvalue_y _returnvalue_z) (`KismetMathLibrary.BreakVector` (`SplineComponent.GetLocationAtDistanceAlongSpline` (`self.SelectedSpline`) _output "Local")))
    (`SceneComponent.K2_SetRelativeLocation` (`BlueprintMapLibrary.Map_Find` (`self.CubeList`) _index) (`KismetMathLibrary.MakeVector` _returnvalue_x _returnvalue_y (+ _returnvalue_z 5.0)) false false)
    (if (`self.IsLooping`)
      (if (> _output (`SplineComponent.GetSplineLength` (`self.SelectedSpline`)))
        (`KismetArrayLibrary.Array_Set` (`self.Distance`) _index)))))

(fn `AddSquareMesh`
  (bind _squarespline (`self.SquareSpline`))
  (for _index (range 4)
    (bind _returnvalue (`AddComponent|NODE_AddStaticMeshComponent-5`))
    (bind _returnvalue_2 (`SplineComponent.GetLocationAtSplinePoint` _squarespline _index "Local"))
    (`SceneComponent.K2_SetRelativeLocation` _returnvalue (/ (+ _returnvalue_2 (`SplineComponent.GetLocationAtSplinePoint` _squarespline (+ _index 1) "Local")) 2) false false)
    (`SceneComponent.SetRelativeScale3D` _returnvalue (1.0 1.0 20.0))
    (if (== (mod _index 2) 0)
      (`SceneComponent.K2_SetRelativeRotation` _returnvalue (struct :`Pitch` 90.0) false false)
      (else
        (`SceneComponent.K2_SetRelativeRotation` _returnvalue (struct :`Pitch` 90.0 :`Roll` 90.0) false false)))
    (bind _returnvalue_3 (`AddComponent|NODE_AddStaticMeshComponent-7`))
    (`SceneComponent.K2_SetRelativeLocation` _returnvalue_3 _returnvalue_2 false false)))

(fn `Get_End_Pos`
  (params (Input :type Integer))
  (returns (Position :type "Vector Structure") (Tangent :type "Vector Structure"))
  (bind _squarespline (`self.SquareSpline`))
  (bind _returnvalue (* (+ Input 1) (`self.SectionLength`)))
  (return (`SplineComponent.GetLocationAtDistanceAlongSpline` _squarespline _returnvalue "Local") (`KismetMathLibrary.ClampVectorSize` (`SplineComponent.GetTangentAtDistanceAlongSpline` _squarespline _returnvalue "Local") 0.0 (`self.SectionLength`))))

(fn `Get_Start_Pos`
  (params (Index :type Integer))
  (returns (Position :type "Vector Structure") (Tangent :type "Vector Structure"))
  (bind _squarespline (`self.SquareSpline`))
  (bind _returnvalue (* Index (`self.SectionLength`)))
  (return (`SplineComponent.GetLocationAtDistanceAlongSpline` _squarespline _returnvalue "Local") (`KismetMathLibrary.ClampVectorSize` (`SplineComponent.GetTangentAtDistanceAlongSpline` _squarespline _returnvalue "Local") 0.0 (`self.SectionLength`))))

(fn `SetDistance`
  (bind _numofcubes (`self.NumOfCubes`))
  (for _index (range (+ _numofcubes 1))
    (`KismetArrayLibrary.Array_Set` (`self.Distance`) _index (* _index (/ (`SplineComponent.GetSplineLength` (`self.SelectedSpline`)) (+ _numofcubes 1))))))

(fn `UserConstructionScript`)