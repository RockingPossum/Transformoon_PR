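; Platformer rotating obstacle that circles cube meshes along a spline alongside a ring of long, rotating meshes.
; BeginPlay spawns both sets, spacing cubes by spline distance and fanning the long meshes at even yaw steps.
; Tick advances the cubes, wrapping when looping, and yaws the meshes at a rate derived from spline length and speed to match one lap.
; Spline-mesh building code in the construction script is disconnected.
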(event `self.ReceiveBeginPlay`
  (set `self.SelectedSpline` (`self.CircleSpline`))
  (`self.CircleMesh`)
  (set `self.BehindSplineMesh` true)
  (set `self.RotationSpeed` (/ 360.0 (/ (`SplineComponent.GetSplineLength` (`self.CircleSpline`)) (`self.Speed`))))
  ;[1 1 1] Add Cube
  (bind _result (`/Engine/EditorBlueprintResources/StandardMacros.DecrementInt` (`self.NumOfCubes`))
    (:`  `
      (for _index (range (+ _result 1))
        (bind _returnvalue (`AddComponent|NODE_AddStaticMeshComponent-0` :`RelativeTransform` (`KismetMathLibrary.MakeTransform` (0.0 0.0 0.0) (struct :`Pitch` 90.0) (0.8 0.8 0.8))))
        (`BlueprintMapLibrary.Map_Add` (`self.CubeList`) _index _returnvalue)
        (`KismetArrayLibrary.Array_Add` (`self.Distance`))
        (`self.SetDistance`)))))

(event `self.ReceiveTick`
  (params (DeltaSeconds :type "Float (single-precision)"))
  (bind _distance (`self.Distance`))
  (`|ExecutionSequence`
    (:`then_0`
      ;[1 1 1] CubeMovement
      (for _index (range (+ (`self.NumOfCubes`) 1))
        (bind _output (`|GetArrayItem` _distance _index))
        (`KismetArrayLibrary.Array_Set` _distance _index (+ (* DeltaSeconds (`self.Speed`)) _output))
        (bind (_returnvalue_x _returnvalue_y _returnvalue_z) (`KismetMathLibrary.BreakVector` (`SplineComponent.GetLocationAtDistanceAlongSpline` (`self.SelectedSpline`) _output "Local")))
        (`SceneComponent.K2_SetRelativeLocation` (`BlueprintMapLibrary.Map_Find` (`self.CubeList`) _index) (`KismetMathLibrary.MakeVector` _returnvalue_x _returnvalue_y (+ _returnvalue_z 35.0)) false false)
        (if (`self.IsLooping`)
          (if (> _output (`SplineComponent.GetSplineLength` (`self.SelectedSpline`)))
            (`KismetArrayLibrary.Array_Set` (`self.Distance`) _index)))))
    (:`then_1`
      ;[1 1 1] CircleMeshMovement
      (if (`self.BehindSplineMesh`)
        (for _array_element (`self.CircleMeshes`)
          (`SceneComponent.K2_AddRelativeRotation` _array_element (`KismetMathLibrary.MakeRotator` 0.0 0.0 (* (* DeltaSeconds (`self.RotationSpeed`)) -1.0)) false false))))))

(fn `CircleMesh`
  (for _index (range (+ (`self.NumOfCubes`) 1))
    (bind _returnvalue (`AddComponent|NODE_AddStaticMeshComponent-8`))
    (`SceneComponent.K2_SetRelativeTransform` _returnvalue (`KismetMathLibrary.MakeTransform` (0.0 -100.0 0.0) (`KismetMathLibrary.MakeRotator` 90.0 0.0 (* _index (/ 360.0 (`KismetMathLibrary.Conv_IntToDouble` (`self.NumOfCubes`))))) (1.0 1.0 40.0)) false false)
    (`KismetArrayLibrary.Array_Add` (`self.CircleMeshes`) _returnvalue)))

(fn `SetDistance`
  (bind _numofcubes (`self.NumOfCubes`))
  (for _index (range (+ _numofcubes 1))
    (`KismetArrayLibrary.Array_Set` (`self.Distance`) _index (* _index (/ (`SplineComponent.GetSplineLength` (`self.SelectedSpline`)) (+ _numofcubes 1))))))

(fn `UserConstructionScript`)