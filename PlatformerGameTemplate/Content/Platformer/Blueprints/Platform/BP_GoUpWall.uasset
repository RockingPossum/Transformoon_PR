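; Platformer actor that runs a looping stream of meshes rising from a Bottom volume to a Top volume.
; BeginPlay spawns meshes at intervals derived from volume distance, speed and count, and Tick moves them upward.
; Meshes overlapping Top are recycled to random points within Bottom instead of being respawned.
; Random placement retries until horizontally clear of the previous mesh on Y, tracked through a wrapping overlap counter.
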(event `self.ReceiveBeginPlay`
  (bind _meshes (`self.Meshes`))
  (`self.FindDuration`)
  (bind _returnvalue (`self.Random Start Location` (`|GetArrayItem` _meshes (`KismetArrayLibrary.Array_LastIndex` _meshes)) :!label _label))
  (bind _returnvalue_2 (`AddComponent|NODE_AddStaticMeshComponent-0` :`RelativeTransform` (`KismetMathLibrary.MakeTransform` _returnvalue (struct) (2.0 2.0 2.0))))
  (`KismetArrayLibrary.Array_Add` (`self.Meshes`) _returnvalue_2)
  (bind _result (`/Engine/EditorBlueprintResources/StandardMacros.IncrementInt` (`self.SpawnedMesh`))
    (:`  `
      (if (< _result (`self.NumOfMesh`))
        (`KismetSystemLibrary.Delay` (`self.Duration`))
        (goto _label)))))

(event `self.ReceiveTick`
  (params (DeltaSeconds :type "Float (single-precision)"))
  (for _array_element (`self.Meshes`)
    (`SceneComponent.K2_AddLocalOffset` _array_element (`KismetMathLibrary.MakeVector` 0.0 0.0 (* DeltaSeconds (`self.Speed`))) false false)))

(event `self.Top.OnComponentBeginOverlap`
  (params (OverlappedComponent :type "PrimitiveComponent Object Reference") (OtherActor :type "Actor Object Reference") (OtherComp :type "PrimitiveComponent Object Reference") (OtherBodyIndex :type Integer) (bFromSweep :type Boolean) (SweepResult :type "HitResult Structure (by ref)"))
  (bind _numofmesh (`self.NumOfMesh`))
  (if (== (`ActorComponent.GetOwner` OtherComp) self)
    (bind _returnvalue (`self.Random Start Location` (`|GetArrayItem` (`self.Meshes`) (`KismetMathLibrary.FTrunc` (`KismetMathLibrary.FMod` (`KismetMathLibrary.Conv_IntToDouble` (- (+ (`self.OverlapCounter`) _numofmesh) 1)) (`KismetMathLibrary.Conv_IntToDouble` _numofmesh))))))
    (`SceneComponent.K2_SetRelativeLocation` OtherComp _returnvalue false false)
    (`/Engine/EditorBlueprintResources/StandardMacros.IncrementInt` (`self.OverlapCounter`))))

(fn `FindDuration`
  (set `self.Duration` (/ (/ (`KismetMathLibrary.Vector_Distance` (`KismetSystemLibrary.GetComponentBounds` (`self.Top`)) (`KismetSystemLibrary.GetComponentBounds` (`self.Bottom`))) (`self.Speed`)) (`self.NumOfMesh`))))

(fn `Random Start Location`
  (params (LastComponent :type "StaticMeshComponent Object Reference"))
  (returns (ReturnValue :type "Vector Structure"))
  (locals (NewLocalVar_0 :type "Vector Structure" :default (0.0 0.0 0.0)))
  (bind _bottom (`self.Bottom`))
  (bind (_relativelocation_x _relativelocation_y) (`KismetMathLibrary.BreakVector` (`SceneComponent.RelativeLocation` LastComponent)))
  (bind (_origin _boxextent) (`KismetSystemLibrary.GetComponentBounds` _bottom))
  (bind _output_get (set `local.NewLocalVar_0` (+ (`SceneComponent.RelativeLocation` _bottom) (`KismetMathLibrary.MakeVector` (`KismetMathLibrary.RandomFloatInRange` (* (.x _boxextent) -1.0) (.x _boxextent)) (`KismetMathLibrary.RandomFloatInRange` (* (.y _boxextent) -1.0) (.y _boxextent)) (`KismetMathLibrary.RandomFloatInRange` (* (.z _boxextent) -1.0) (.z _boxextent)))) :!label _label))
  (`/Engine/EditorBlueprintResources/StandardMacros.IsValid` LastComponent
    (:`Is Valid`
      (if (> (`KismetMathLibrary.Abs` (- (.y _output_get) _relativelocation_y)) 100.0)
        _
        (else
          (goto _label))))
    (:`Is Not Valid`
      _))
  (return (`local.NewLocalVar_0`)))

(fn `UserConstructionScript`)