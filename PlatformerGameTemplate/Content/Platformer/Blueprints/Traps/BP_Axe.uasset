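; BP_Axe is a swinging trap for the platformer that damages the player character on contact.
; On BeginPlay a looping timeline offsets the Saw2 component's pitch from its starting rotation to animate the swing.
; When Saw2 begins overlapping a BP_Character, it waits one tick as a bug fix, then calls SetHealth with a negative value on that character.
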(event `self.ReceiveBeginPlay`
  (bind (_rotation_roll _rotation_pitch _rotation_yaw) (`KismetMathLibrary.BreakRotator` (`self.Rotation`)))
  (`|ExecutionSequence`
    (:`then_0`
      (set `self.Rotation` (`SceneComponent.K2_GetComponentRotation` (`self.Saw2`)))
      (bind (_direction _newtrack_0) (`Timeline|Timeline_3` :!label _label)
        (:`Update`
          (`SceneComponent.K2_SetWorldRotation` (`self.Saw2`) (`KismetMathLibrary.MakeRotator` _rotation_roll (+ _newtrack_0 _rotation_pitch) _rotation_yaw) false false))
        (:`Finished`
          (goto _label :!via `PlayFromStart`))))))

(event `self.Saw2.OnComponentBeginOverlap`
  (params (OverlappedComponent :type "PrimitiveComponent Object Reference") (OtherActor :type "Actor Object Reference") (OtherComp :type "PrimitiveComponent Object Reference") (OtherBodyIndex :type Integer) (bFromSweep :type Boolean) (SweepResult :type "HitResult Structure (by ref)"))
  (bind _asbp_character (cast `/Game/Platformer/Blueprints/BP_Character` OtherActor))
  ;[1 1 1] Bug Fix Dont Destroy
  (`KismetSystemLibrary.DelayUntilNextTick`)
  (`/Game/Platformer/Blueprints/BP_Character.SetHealth` _asbp_character -1.0))

(fn `UserConstructionScript`)