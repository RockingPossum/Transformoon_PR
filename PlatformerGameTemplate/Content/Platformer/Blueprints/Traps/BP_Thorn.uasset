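; Thorn trap for a platformer that moves vertically in a repeating cycle and harms the player character on contact.
; BeginPlay caches the scene component's world location, then a Timeline offsets its Z each update and restarts from the start when finished.
; When ThornB overlaps a BP_Character, it waits one tick, noted as a bug fix, then calls SetHealth with a negative value.
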(event `self.ReceiveBeginPlay`
  (bind (_transform_x _transform_y _transform_z) (`KismetMathLibrary.BreakVector` (`self.Transform`)))
  (set `self.Transform` (`SceneComponent.K2_GetComponentLocation` (`self.Scene`)))
  (`TimelineComponent.SetPlayRate` (`self.Timeline_0`) 1.0)
  (bind (_direction _newtrack_0) (`Timeline|Timeline_0` :!label _label)
    (:`Update`
      (`SceneComponent.K2_SetWorldLocation` (`self.Scene`) (`KismetMathLibrary.MakeVector` _transform_x _transform_y (+ _newtrack_0 _transform_z)) false false))
    (:`Finished`
      (goto _label :!via `PlayFromStart`))))

(event `self.ThornB.OnComponentBeginOverlap`
  (params (OverlappedComponent :type "PrimitiveComponent Object Reference") (OtherActor :type "Actor Object Reference") (OtherComp :type "PrimitiveComponent Object Reference") (OtherBodyIndex :type Integer) (bFromSweep :type Boolean) (SweepResult :type "HitResult Structure (by ref)"))
  (bind _asbp_character (cast `/Game/Platformer/Blueprints/BP_Character` OtherActor))
  ;[1 1 1] Bug Fix Dont Destroy
  (`KismetSystemLibrary.DelayUntilNextTick`)
  (`/Game/Platformer/Blueprints/BP_Character.SetHealth` _asbp_character -1.0))

(fn `UserConstructionScript`)