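; BP_SpinningWheel_C is a platformer trap that continuously spins two saw components, Saw2 and Saw3.
; On BeginPlay, each saw gets its own timeline that adds an animated yaw offset to a cached world rotation and restarts when finished.
; Both saws write to the same Rotation variable, so Saw3's starting rotation overwrites Saw2's and becomes the base for both.
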(event `self.ReceiveBeginPlay`
  (bind (_rotation_roll _rotation_pitch _rotation_yaw) (`KismetMathLibrary.BreakRotator` (`self.Rotation`)))
  (bind (_rotation_roll_2 _rotation_pitch_2 _rotation_yaw_2) (`KismetMathLibrary.BreakRotator` (`self.Rotation`)))
  (`|ExecutionSequence`
    (:`then_0`
      (set `self.Rotation` (`SceneComponent.K2_GetComponentRotation` (`self.Saw2`)))
      (bind (_direction _newtrack_0) (`Timeline|Timeline_3` :!label _label)
        (:`Update`
          (`SceneComponent.K2_SetWorldRotation` (`self.Saw2`) (`KismetMathLibrary.MakeRotator` _rotation_roll _rotation_pitch (+ _newtrack_0 _rotation_yaw)) false false))
        (:`Finished`
          (goto _label :!via `PlayFromStart`))))
    (:`then_1`
      (set `self.Rotation` (`SceneComponent.K2_GetComponentRotation` (`self.Saw3`)))
      (bind (_direction_2 _newtrack_0_2) (`Timeline|Timeline_0` :!label _label_2)
        (:`Update`
          (`SceneComponent.K2_SetWorldRotation` (`self.Saw3`) (`KismetMathLibrary.MakeRotator` _rotation_roll_2 _rotation_pitch_2 (+ _newtrack_0_2 _rotation_yaw_2)) false false))
        (:`Finished`
          (goto _label_2 :!via `PlayFromStart`))))))

(fn `UserConstructionScript`)